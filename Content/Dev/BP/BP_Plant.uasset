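; Grabbable VR plant that can be planted in a pot or collected into the player's backpack.
; On drop or Plant, it finds the nearest BP_Pot and, within PlantRange, snaps upright onto it and swaps its mesh to Mecha_duck after a delay; otherwise it simulates physics.
; Overlapping the XR pawn's Mochila while OnHold is set increments the inventory's plant count and destroys the plant.
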(event `Plant`
  (bind _plantmesh (`self.PlantMesh`))
  (bind (_nearest_actor _distance) (`self.GetNearestActorOfClass` "/Game/Dev/BP/BP_Pot.BP_Pot_C" :!label _label))
  (if (< _distance (`self.PlantRange`))
    (`PrimitiveComponent.SetSimulatePhysics` _plantmesh false)
    (`SceneComponent.K2_SetWorldLocation` _plantmesh (`self.K2_GetActorLocation` _nearest_actor) false true)
    (`SceneComponent.K2_SetRelativeRotation` :`self` (`self.PlantMesh`))
    (`KismetSystemLibrary.Delay` 10.0)
    (`StaticMeshComponent.SetStaticMesh` (`self.PlantMesh`) "/Game/Fab/mecha_duck/mecha_duck/StaticMeshes/mecha_duck.mecha_duck")
    (else
      (`PrimitiveComponent.SetSimulatePhysics` (`self.PlantMesh`) true))))

(event `self.BP_GrabComponent.OnDropped`
  (goto _label))

(event `self.PlantMesh.OnComponentBeginOverlap`
  (params (OverlappedComponent :type "PrimitiveComponent Object Reference") (OtherActor :type "Actor Object Reference") (OtherComp :type "PrimitiveComponent Object Reference") (OtherBodyIndex :type Integer) (bFromSweep :type Boolean) (SweepResult :type "HitResult Structure (by ref)"))
  (bind _returnvalue (`GameplayStatics.GetActorOfClass` "/Game/XRFramework/Blueprints/BP_XRPawn.BP_XRPawn_C"))
  (if (and (`self.OnHold`) (== (`/Game/XRFramework/Blueprints/BP_XRPawn.Mochila` _returnvalue) OtherComp))
    (bind _ac_inventory (`/Game/XRFramework/Blueprints/BP_XRPawn.AC_Inventory` _returnvalue))
    (set `/Game/Dev/BP/AC_Inventory.PlantCount` (+ (`/Game/Dev/BP/AC_Inventory.PlantCount` _ac_inventory) 1) _ac_inventory)
    (`self.K2_DestroyActor`)))

(fn `GetNearestActorOfClass`
  (params (ActorClass :type "Actor Class Reference"))
  (returns (`Nearest Actor` :type "Actor Object Reference") (Distance :type "Float (double-precision)"))
  (locals (Loc_ShortestDistance :type "Float (double-precision)" :default 99999999.0) (Loc_NearestActor :type "Actor Object Reference"))
  (bind _outactors (`GameplayStatics.GetAllActorsOfClass` ActorClass))
  (for _array_element _outactors
    (bind _returnvalue (`KismetMathLibrary.Vector_Distance` (`self.K2_GetActorLocation` _array_element) (`SceneComponent.K2_GetComponentLocation` (`self.PlantMesh`))))
    (if (< _returnvalue (`local.Loc_ShortestDistance`))
      (set `local.Loc_NearestActor` _array_element)
      (set `local.Loc_ShortestDistance` _returnvalue)))
  (return (`local.Loc_NearestActor`) (`local.Loc_ShortestDistance`)))

(fn `UserConstructionScript`)