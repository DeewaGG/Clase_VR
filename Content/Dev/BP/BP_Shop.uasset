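; BP_Shop is a shop trigger that automatically sells a plant to the XR pawn when it enters.
; On Box1 begin overlap, it checks the pawn's ACInventory Money against a hardcoded minimum.
; With enough money, it spawns a BP_Plant at the pawn's location and deducts that plant's Value.
; The affordability threshold is independent of the Value actually charged.
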(event `self.Box1.OnComponentBeginOverlap`
  (params (OverlappedComponent :type "PrimitiveComponent Object Reference") (OtherActor :type "Actor Object Reference") (OtherComp :type "PrimitiveComponent Object Reference") (OtherBodyIndex :type Integer) (bFromSweep :type Boolean) (SweepResult :type "HitResult Structure (by ref)"))
  (bind _asbp_xrpawn (cast `/Game/XRFramework/Blueprints/BP_XRPawn` OtherActor))
  (if (not (< (`/Game/Dev/BP/AC_Inventory.Money` (`/Game/XRFramework/Blueprints/BP_XRPawn.AC_Inventory` _asbp_xrpawn)) 250))
    (bind _returnvalue (`|SpawnActorFromClass` "/Game/Dev/BP/BP_Plant.BP_Plant_C" (`KismetMathLibrary.MakeTransform` (`self.K2_GetActorLocation` _asbp_xrpawn)) "Undefined" "MultiplyWithRoot" null null))
    (bind _ac_inventory (`/Game/XRFramework/Blueprints/BP_XRPawn.AC_Inventory` _asbp_xrpawn))
    (set `/Game/Dev/BP/AC_Inventory.Money` (- (`/Game/Dev/BP/AC_Inventory.Money` _ac_inventory) (`/Game/Dev/BP/BP_Plant.Value` _returnvalue)) _ac_inventory)))

(fn `UserConstructionScript`)