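; BP_Mecha is a drivable mech for the XR pawn, which snaps onto a seat target when it overlaps the entrance trigger.
; Two pairs of forward/backward collision volumes act as controls, setting move or rotate flags and directions while the pawn overlaps them.
; Tick offsets the mech along the player pawn's forward vector, without sweep, and applies yaw rotation, both scaled by speed and delta time.
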(event `self.Entrance.OnComponentBeginOverlap`
  (params (OverlappedComponent :type "PrimitiveComponent Object Reference") (OtherActor :type "Actor Object Reference") (OtherComp :type "PrimitiveComponent Object Reference") (OtherBodyIndex :type Integer) (bFromSweep :type Boolean) (SweepResult :type "HitResult Structure (by ref)"))
  (bind _asbp_xrpawn (cast `/Game/XRFramework/Blueprints/BP_XRPawn` OtherActor))
  (`self.K2_AttachToComponent` _asbp_xrpawn (`self.TP_Target`) "None" "SnapToTarget" "SnapToTarget" "KeepWorld" true))

(event `self.Backwards_Coll.OnComponentBeginOverlap`
  (params (OverlappedComponent :type "PrimitiveComponent Object Reference") (OtherActor :type "Actor Object Reference") (OtherComp :type "PrimitiveComponent Object Reference") (OtherBodyIndex :type Integer) (bFromSweep :type Boolean) (SweepResult :type "HitResult Structure (by ref)"))
  (cast `/Game/XRFramework/Blueprints/BP_XRPawn` OtherActor)
  (set `self.bMoving` true)
  (set `self.MovingDirection` -1))

(event `self.Forward_Coll1.OnComponentBeginOverlap`
  (params (OverlappedComponent :type "PrimitiveComponent Object Reference") (OtherActor :type "Actor Object Reference") (OtherComp :type "PrimitiveComponent Object Reference") (OtherBodyIndex :type Integer) (bFromSweep :type Boolean) (SweepResult :type "HitResult Structure (by ref)"))
  (cast `/Game/XRFramework/Blueprints/BP_XRPawn` OtherActor)
  (set `self.bRotating` true)
  (set `self.RotatorDirection` 1))

(event `self.Backwards_Coll1.OnComponentBeginOverlap`
  (params (OverlappedComponent :type "PrimitiveComponent Object Reference") (OtherActor :type "Actor Object Reference") (OtherComp :type "PrimitiveComponent Object Reference") (OtherBodyIndex :type Integer) (bFromSweep :type Boolean) (SweepResult :type "HitResult Structure (by ref)"))
  (cast `/Game/XRFramework/Blueprints/BP_XRPawn` OtherActor)
  (set `self.bRotating` true)
  (set `self.RotatorDirection` -1))

(event `self.Forward_Coll.OnComponentBeginOverlap`
  (params (OverlappedComponent :type "PrimitiveComponent Object Reference") (OtherActor :type "Actor Object Reference") (OtherComp :type "PrimitiveComponent Object Reference") (OtherBodyIndex :type Integer) (bFromSweep :type Boolean) (SweepResult :type "HitResult Structure (by ref)"))
  (cast `/Game/XRFramework/Blueprints/BP_XRPawn` OtherActor)
  (set `self.bMoving` true)
  (set `self.MovingDirection` 1))

(event `self.Forward_Coll1.OnComponentEndOverlap`
  (params (OverlappedComponent :type "PrimitiveComponent Object Reference") (OtherActor :type "Actor Object Reference") (OtherComp :type "PrimitiveComponent Object Reference") (OtherBodyIndex :type Integer))
  (cast `/Game/XRFramework/Blueprints/BP_XRPawn` OtherActor)
  (set `self.bRotating` false :!label _label))

(event `self.Backwards_Coll.OnComponentEndOverlap`
  (params (OverlappedComponent :type "PrimitiveComponent Object Reference") (OtherActor :type "Actor Object Reference") (OtherComp :type "PrimitiveComponent Object Reference") (OtherBodyIndex :type Integer))
  (cast `/Game/XRFramework/Blueprints/BP_XRPawn` OtherActor)
  (set `self.bMoving` false :!label _label_2))

(event `self.Forward_Coll.OnComponentEndOverlap`
  (params (OverlappedComponent :type "PrimitiveComponent Object Reference") (OtherActor :type "Actor Object Reference") (OtherComp :type "PrimitiveComponent Object Reference") (OtherBodyIndex :type Integer))
  (cast `/Game/XRFramework/Blueprints/BP_XRPawn` OtherActor)
  (goto _label_2))

(event `self.Backwards_Coll1.OnComponentEndOverlap`
  (params (OverlappedComponent :type "PrimitiveComponent Object Reference") (OtherActor :type "Actor Object Reference") (OtherComp :type "PrimitiveComponent Object Reference") (OtherBodyIndex :type Integer))
  (cast `/Game/XRFramework/Blueprints/BP_XRPawn` OtherActor)
  (goto _label))

(event `self.ReceiveTick`
  (params (DeltaSeconds :type "Float (single-precision)"))
  (bind _returnvalue (`self.GetActorForwardVector` (`GameplayStatics.GetPlayerPawn` 0)))
  (`|ExecutionSequence`
    (:`then_0`
      (if (`self.bMoving`)
        (`self.K2_AddActorWorldOffset` (* (`KismetMathLibrary.SelectVector` _returnvalue (`KismetMathLibrary.NegateVector` _returnvalue) (== (`self.MovingDirection`) 1)) (`self.MovSpeed`) (`GameplayStatics.GetWorldDeltaSeconds`)))))
    (:`then_1`
      (if (`self.bRotating`)
        (`self.K2_AddActorWorldRotation` (`KismetMathLibrary.MakeRotator` 0.0 0.0 (* (`self.RotatorDirection`) (`self.RotSpeed`) (`GameplayStatics.GetWorldDeltaSeconds`))))))))

(fn `UserConstructionScript`)